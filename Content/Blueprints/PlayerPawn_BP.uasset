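; Player pawn that launches a projectile ball from a touch swipe, forwarding touch and possession events to UTC manager components.
; Both successful and failed swipes spawn a ball, aimed by swipe direction combined with the actor's right vector.
; Swipe length, not elapsed time as comments claim, scales the forward and upward launch velocity.
; Each launch destroys the previous ball and decrements the ball count in LimitedGameModeBase.
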(event `self.SwipeComponent.On Swipe Gesture Success`
  (params (`Start Location` :type "Vector Structure") (`End Location` :type "Vector Structure") (Direction :type "Vector Structure") (`Elapsed Time` :type "Timespan Structure") (`Swipe Direction` :type "/Game/TouchComponents/Core/ESwipeDirection Enum" :default "NewEnumerator0"))
  (`self.NewMacro_0` `Start Location` `End Location` Direction `Elapsed Time`))

(event `InputTouch`
  (params (Location :type "Vector Structure") (FingerIndex :type "ETouchIndex Enum"))
  ;[1 0 0] Pass required events to all UTC components
  (:`Pressed`
    (`/Game/TouchComponents/Core/MacroLibrary.UTC Touch Input Manager` Location FingerIndex :!label _label))
  (:`Released`
    (goto _label :!via `Released`))
  (:`Moved`
    (goto _label :!via `Moved`)))

(event `self.SwipeComponent.On Swipe Gesture Fail`
  (params (`Start Location` :type "Vector Structure") (`End Location` :type "Vector Structure") (Direction :type "Vector Structure") (`Elapsed Time` :type "Timespan Structure") (`Swipe Direction` :type "/Game/TouchComponents/Core/ESwipeDirection Enum" :default "NewEnumerator0"))
  (`self.NewMacro_0` `Start Location` `End Location` Direction `Elapsed Time`))

(event `self.ReceivePossessed`
  (params (NewController :type "Controller Object Reference"))
  ;[1 0 0] Pass required events to all UTC components
  (`/Game/TouchComponents/Core/MacroLibrary.UTC Pawn Possesion Manager` NewController (stale `self.ReceiveUnpossessed` OldController) :!label _label_2))

(event `self.ReceiveUnpossessed`
  (params (OldController :type "Controller Object Reference"))
  ;[1 0 0] Pass required events to all UTC components
  (goto _label_2 :!via `Unpossesed`))

(fn `UserConstructionScript`)